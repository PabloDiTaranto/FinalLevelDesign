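; Moving platform actor that shuttles back and forth between its Init and End components, starting toward End.
; Move, started on BeginPlay, offsets the platform toward the target by Speed and delta time, re-calling itself through a zero Delay instead of Tick.
; Within a small distance of the target, it flips direction and pauses for WaitTime.
; Helper events snap the platform to Init or set either endpoint to its current position.
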(event Custom|SetToInit
  (Transformation|SetWorldLocation (Variables|Default|GetPlatform) (Transformation|GetWorldLocation (Variables|Default|GetInit)) false false))

(event Custom|SetEndToCurrentPlatformPos
  (Transformation|SetWorldLocation (Variables|Default|GetEnd) (Transformation|GetWorldLocation (Variables|Default|GetPlatform)) false false))

(event Custom|SetInitToCurrentPlatformPos
  (Transformation|SetWorldLocation (Variables|Default|GetInit) (Transformation|GetWorldLocation (Variables|Default|GetPlatform)) false false))

(event Custom|Move
  (Transformation|AddLocalOffset (Variables|Default|GetPlatform) (* (Math|Vector|Normalize (- (Variables|/Script/Engine.SceneComponent|GetRelativeLocation (select (Variables|Default|GetToInit) (Variables|Default|GetInit) (Variables|Default|GetEnd))) (Variables|/Script/Engine.SceneComponent|GetRelativeLocation (Variables|Default|GetPlatform)))) (* (Utilities|Time|GetWorldDeltaSeconds) (Variables|Configuration|GetSpeed))) false false)
  (if (< (Math|Vector|VectorLength (- (Transformation|GetWorldLocation (select (Variables|Default|GetToInit) (Variables|Default|GetInit) (Variables|Default|GetEnd))) (Transformation|GetWorldLocation (Variables|Default|GetPlatform)))) 1e+01)
    (if (Variables|Default|GetToInit)
      (Variables|Default|SetToInit false)
      (else
        (Variables|Default|SetToInit true)))
    (Utilities|FlowControl|Delay (Variables|Configuration|GetWaitTime))
    (CallFunction|Move)
    (else
      (Utilities|FlowControl|Delay 0.0)
      (CallFunction|Move))))

(event EventBeginPlay
  (Variables|Default|SetToInit false)
  (CallFunction|Move))

(fn ConstructionScript)