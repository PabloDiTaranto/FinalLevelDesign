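; Level actor for a moving platform that shuttles continuously between its Init and End points, starting on BeginPlay.
; The MovePlatform timeline lerps the Platform's world location between the two points without sweeping.
; On finish it waits WaitTime, then uses the timeline direction to play in reverse or forward again.
; Helper events snap the platform to Init or set either endpoint to the platform's current position.
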(event Custom|SetToInit
  (Transformation|SetWorldLocation (Variables|Default|GetPlatform) (Transformation|GetWorldLocation (Variables|Default|GetInit)) false false))

(event Custom|MoveToEnd
  (bind (_direction _newtrack_0) (Timeline|MovePlatform PlayFromStart)
    (:Update
      (Transformation|SetWorldLocation (Variables|Default|GetPlatform) (Math|Vector|Lerp(Vector) (Transformation|GetWorldLocation (Variables|Default|GetInit)) (Transformation|GetWorldLocation (Variables|Default|GetEnd)) _newtrack_0) false false))
    (:Finished
      (Utilities|FlowControl|Delay (Variables|Configuration|GetWaitTime))
      (switch Utilities|FlowControl|Switch|SwitchonETimelineDirection _direction
        (:Forward
          (CallFunction|MovetoInit))
        (:Backward
          (CallFunction|MovetoEnd))))))

(event Custom|MoveToInit
  (bind (_direction _newtrack_0) (Timeline|MovePlatform ReverseFromEnd)
    (:Update
      (Transformation|SetWorldLocation (Variables|Default|GetPlatform) (Math|Vector|Lerp(Vector) (Transformation|GetWorldLocation (Variables|Default|GetInit)) (Transformation|GetWorldLocation (Variables|Default|GetEnd)) _newtrack_0) false false))
    (:Finished
      (Utilities|FlowControl|Delay (Variables|Configuration|GetWaitTime))
      (switch Utilities|FlowControl|Switch|SwitchonETimelineDirection _direction
        (:Forward
          (CallFunction|MovetoInit))
        (:Backward
          (CallFunction|MovetoEnd))))))

(event Custom|SetEndToCurrentPlatformPos
  (Transformation|SetWorldLocation (Variables|Default|GetEnd) (Transformation|GetWorldLocation (Variables|Default|GetPlatform)) false false))

(event Custom|SetInitToCurrentPlatformPos
  (Transformation|SetWorldLocation (Variables|Default|GetInit) (Transformation|GetWorldLocation (Variables|Default|GetPlatform)) false false))

(event EventBeginPlay
  (CallFunction|MovetoEnd))

(fn ConstructionScript)