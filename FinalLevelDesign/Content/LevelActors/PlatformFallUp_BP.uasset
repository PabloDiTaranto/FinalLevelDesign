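; Platform actor that endlessly cycles between an Up and a Down scene marker, optionally starting at the bottom via StartDown.
; GoDown waits TimeToGoDown, shakes the platform's rotation with a timeline as a warning, resets it, then lerps it down before calling GoUp.
; GoUp waits TimeToGoUp, lerps it back up with its own timeline and calls GoDown again.
; Platform and Collision move together, but only the Platform shakes.
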(event Custom|GoDown
  (Utilities|FlowControl|Delay (Variables|Configuration|GetTimeToGoDown))
  (bind _newtrack_0 (Timeline|ShakePlatform PlayFromStart)
    (:Update
      (Transformation|SetRelativeRotation (Variables|Default|GetPlatform) (Math|Rotator|Lerp(Rotator) "1.000000,-2.000000,-1.000000" "-1.000000,2.000000,1.000000" _newtrack_0 true) false false))
    (:Finished
      (Transformation|SetRelativeRotation (Variables|Default|GetPlatform) "0, 0, 0" false false)
      (bind _newtrack_0_2 (Timeline|MoveDown PlayFromStart)
        (:Update
          (Transformation|SetWorldLocation (Variables|Default|GetPlatform) (Math|Vector|Lerp(Vector) (Transformation|GetWorldLocation (Variables|Default|GetUp)) (Transformation|GetWorldLocation (Variables|Default|GetDown)) _newtrack_0_2) false false))
        (:Finished
          (CallFunction|GoUp))))))

(event Custom|GoUp
  (Utilities|FlowControl|Delay (Variables|Configuration|GetTimeToGoUp))
  (bind _newtrack_0 (Timeline|MovePlatformUp PlayFromStart)
    (:Update
      (Transformation|SetWorldLocation (Variables|Default|GetPlatform) (Math|Vector|Lerp(Vector) (Transformation|GetWorldLocation (Variables|Default|GetDown)) (Transformation|GetWorldLocation (Variables|Default|GetUp)) _newtrack_0) false false))
    (:Finished
      (CallFunction|GoDown))))

(event EventBeginPlay
  (if (Variables|Configuration|GetStartDown?)
    (Transformation|SetWorldLocation (Variables|Default|GetPlatform) (Transformation|GetWorldLocation (Variables|Default|GetDown)) false false)
    (CallFunction|GoUp)
    (else
      (CallFunction|GoDown))))

(fn ConstructionScript)