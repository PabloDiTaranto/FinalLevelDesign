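; Spike trap level actor that kills actors implementing MainCharacter_BPI on contact with its damage volume.
; Runs either as a timed loop after a start delay or, with a green floor, when the character overlaps the detection volume.
; Chained timelines partly raise the spikes, pause, thrust them fully up with a sound, then lower them.
; A DoOnce blocks retriggering until the spikes finish lowering.
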(event OnComponentBeginOverlap(PlayerDetection)
  (params (OverlappedComponent :type Primitive%20Component%20Object%20Reference) (OtherActor :type Actor%20Object%20Reference) (OtherComp :type Primitive%20Component%20Object%20Reference) (OtherBodyIndex :type Integer) (bFromSweep :type Boolean) (SweepResult :type Hit%20Result%20Structure%20%28by%20ref%29))
  (if (Utilities|DoesObjectImplementInterface OtherActor "/Game/ThirdPersonBP/Blueprints/MainCharacter_BPI.MainCharacter_BPI_C")
    (Utilities|FlowControl|DoOnce false
      (:Completed
        (CallFunction|UpSpikes)))))

(event OnComponentBeginOverlap(Damage)
  (params (OverlappedComponent :type Primitive%20Component%20Object%20Reference) (OtherActor :type Actor%20Object%20Reference) (OtherComp :type Primitive%20Component%20Object%20Reference) (OtherBodyIndex :type Integer) (bFromSweep :type Boolean) (SweepResult :type Hit%20Result%20Structure%20%28by%20ref%29))
  (if (Utilities|DoesObjectImplementInterface OtherActor "/Game/ThirdPersonBP/Blueprints/MainCharacter_BPI.MainCharacter_BPI_C")
    (Class|MainCharacterBPI|OnDead(Message) OtherActor)))

(event Custom|UpSpikes
  (bind _newtrack_0 (Timeline|StartUp PlayFromStart)
    (:Update
      (Transformation|SetRelativeLocation (Variables|Default|GetSpikes_SpikeTeap_spike_LP_002) (Math|Vector|Lerp(Vector) "0, 0,-40.000000" "0, 0,-20.000000" _newtrack_0) false false))
    (:Finished
      (Utilities|FlowControl|Delay (Variables|Configuration|GetTimeBeforeDamage))
      (Audio|PlaySoundatLocation "/Game/Sounds/Spikes_Cue.Spikes_Cue" (Transformation|GetActorLocation) "0, 0, 0" 1.0 1.0 0.0 0 0 0)
      (bind _newtrack_0_2 (Timeline|GoUp PlayFromStart)
        (:Update
          (Transformation|SetRelativeLocation (Variables|Default|GetSpikes_SpikeTeap_spike_LP_002) (Math|Vector|Lerp(Vector) "0, 0,-20.000000" "0, 0, 0" _newtrack_0_2) false false))
        (:Finished
          (CallFunction|DownSpikes))))))

(event Custom|DownSpikes
  (bind _newtrack_0 (Timeline|Down PlayFromStart)
    (:Update
      (Transformation|SetRelativeLocation (Variables|Default|GetSpikes_SpikeTeap_spike_LP_002) (Math|Vector|Lerp(Vector) "0, 0, 0" "0, 0,-40.000000" _newtrack_0) false false))
    (:Finished
      (if (Variables|Configuration|GetByTime?)
        (Utilities|FlowControl|Delay (Variables|Configuration|GetWaitTime))
        (CallFunction|UpSpikes)
        (else
          (CallFunction|ResetDoOnce))))))

(event Custom|ResetDoOnce
  (Utilities|FlowControl|DoOnce false) ; enters at Reset
)

(event EventBeginPlay
  (if (Variables|Configuration|GetByTime?)
    (Rendering|Material|SetMaterial (Variables|Default|GetSpikes_SpikeTeap_Floor_LP_001) 0 "/Game/AlchemistsHouse/Extra_Assets/M_Floor.M_Floor")
    (Collision|SetCollisionEnabled (Variables|Default|GetPlayerDetection) "NoCollision")
    (Utilities|FlowControl|Delay (Variables|Configuration|GetTimeBeforeStart))
    (CallFunction|UpSpikes)
    (else
      (Rendering|Material|SetMaterial (Variables|Default|GetSpikes_SpikeTeap_Floor_LP_001) 0 "/Game/AlchemistsHouse/Extra_Assets/MI_Floor_Green.MI_Floor_Green"))))

(fn ConstructionScript)