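; PatrolSlime is an enemy character that patrols a looping route and kills the main character on contact.
; On BeginPlay it sets its walk speed, then uses AI MoveTo to walk through the TargetPoints in order, wrapping to the first and advancing even when a move fails.
; Overlapping its DamageArea sends OnDeadMessage to any actor that implements MainCharacter_BPI.
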(event OnComponentBeginOverlap(DamageArea)
  (params (OverlappedComponent :type Primitive%20Component%20Object%20Reference) (OtherActor :type Actor%20Object%20Reference) (OtherComp :type Primitive%20Component%20Object%20Reference) (OtherBodyIndex :type Integer) (bFromSweep :type Boolean) (SweepResult :type Hit%20Result%20Structure%20%28by%20ref%29))
  (if (Utilities|DoesObjectImplementInterface OtherActor "/Game/ThirdPersonBP/Blueprints/MainCharacter_BPI.MainCharacter_BPI_C")
    (Class|MainCharacterBPI|OnDead(Message) OtherActor)))

(event Custom|MoveToNextTargetPoint
  (AI|AIMoveTo self (Transformation|GetActorLocation (Utilities|Array|Get(acopy) (Variables|Configuration|GetTargetPoints) (Variables|Default|GetCurrentPoint))) 0 5.0 false
    (:OnSuccess
      _)
    (:OnFail
      _))
  (bind _output_get (Variables|Default|SetCurrentPoint (+ (Variables|Default|GetCurrentPoint) 1)))
  (if (>= _output_get (Utilities|Array|Length (Variables|Configuration|GetTargetPoints)))
    (Variables|Default|SetCurrentPoint 0))
  (CallFunction|MovetoNextTargetPoint))

(event EventBeginPlay
  (Variables|/Script/Engine.CharacterMovementComponent|SetMaxWalkSpeed (Variables|Character|GetCharacterMovement) (Variables|Configuration|GetSpeed))
  (CallFunction|MovetoNextTargetPoint))

(fn ConstructionScript)