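; BulletSlime_BP is a slime projectile that kills the main character on contact.
; A ProjectileMovement component drives it, with the construction script setting both initial and max speed from the InitialSpeed variable.
; When its Sphere overlaps any actor other than its owner, it sends OnDeadMessage through MainCharacter_BPI to actors implementing that interface, then destroys itself.
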(event OnComponentBeginOverlap(Sphere)
  (params (OverlappedComponent :type Primitive%20Component%20Object%20Reference) (OtherActor :type Actor%20Object%20Reference) (OtherComp :type Primitive%20Component%20Object%20Reference) (OtherBodyIndex :type Integer) (bFromSweep :type Boolean) (SweepResult :type Hit%20Result%20Structure%20%28by%20ref%29))
  (if (not (== OtherActor (Components|GetOwner)))
    (if (Utilities|DoesObjectImplementInterface OtherActor "/Game/ThirdPersonBP/Blueprints/MainCharacter_BPI.MainCharacter_BPI_C")
      (Class|MainCharacterBPI|OnDead(Message) OtherActor))
    (Actor|DestroyActor)))

(event EventBeginPlay)

(fn ConstructionScript
  (bind _projectilemovement (Variables|Default|GetProjectileMovement))
  (bind _output_get (Variables|/Script/Engine.ProjectileMovementComponent|SetInitialSpeed _projectilemovement (Variables|Default|GetInitial%20Speed)))
  (Variables|/Script/Engine.ProjectileMovementComponent|SetMaxSpeed _projectilemovement _output_get))