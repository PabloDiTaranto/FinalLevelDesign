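; SlimeRange_BP is a ranged slime hazard that fires bullets continuously and kills the main character on contact.
; From BeginPlay, the Shoot event spawns a BulletSlime_BP at SpawnPoint with configurable scale and speed, then re-calls itself after a FireRate delay.
; Overlapping its Sphere sends OnDeadMessage to any actor implementing MainCharacter_BPI, avoiding a cast to the character class.
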(event OnComponentBeginOverlap(Sphere)
  (params (OverlappedComponent :type Primitive%20Component%20Object%20Reference) (OtherActor :type Actor%20Object%20Reference) (OtherComp :type Primitive%20Component%20Object%20Reference) (OtherBodyIndex :type Integer) (bFromSweep :type Boolean) (SweepResult :type Hit%20Result%20Structure%20%28by%20ref%29))
  (if (Utilities|DoesObjectImplementInterface OtherActor "/Game/ThirdPersonBP/Blueprints/MainCharacter_BPI.MainCharacter_BPI_C")
    (Class|MainCharacterBPI|OnDead(Message) OtherActor)))

(event Custom|Shoot
  (bind _spawnpoint (Variables|Default|GetSpawnPoint))
  (bind _bulletscale (Variables|Configuration|GetBulletScale))
  (bind _returnvalue (Transformation|GetWorldTransform _spawnpoint))
  (Game|SpawnActorfromClass "/Game/Slime1/BulletSlime_BP.BulletSlime_BP_C" (Math|Transform|MakeTransform (.location _returnvalue) (.rotation _returnvalue) (Math|Vector|MakeVector _bulletscale _bulletscale _bulletscale)) "Undefined" self (Variables|Configuration|GetBulletSpeed) 0)
  (Utilities|FlowControl|Delay (Variables|Configuration|GetFireRate))
  (CallFunction|Shoot))

(event EventBeginPlay
  (CallFunction|Shoot))

(fn ConstructionScript)